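; BP_Weapon is a pickup light weapon that hurts monsters.
; Overlap by BP_TestPlayer attaches it to the mesh's "Light" socket, sets the anim blueprint's IsOnLight and binds to the player's use-item event.
; LightServer, called by OnLightProjectile, toggles the light and trace flags.
; While tracing, Tick runs debug-drawn sphere traces with cycling radius until LightRange, which never resets, reaches its cap, applying point damage to BP_Monster hits.
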(event OnComponentBeginOverlap(SphereCollision)
  (params (OverlappedComponent :type Primitive%20Component%20Object%20Reference) (OtherActor :type Actor%20Object%20Reference) (OtherComp :type Primitive%20Component%20Object%20Reference) (OtherBodyIndex :type Integer) (bFromSweep :type Boolean) (SweepResult :type Hit%20Result%20Structure%20%28by%20ref%29))
  (bind _asbp_test_player (Utilities|Casting|CastToBP_TestPlayer OtherActor))
  (Variables|Default|SetFirstPersonCharacterReference _asbp_test_player)
  (Transformation|AttachComponentToComponent self (Variables|/Script/Engine.Character|GetMesh (Variables|Default|GetFirstPersonCharacterReference)) "Light" "SnapToTarget" "SnapToTarget" "SnapToTarget" true)
  (bind _asabp_mtk_player (Utilities|Casting|CastToABP_MTK_Player (Components|SkeletalMesh|GetAnimInstance (Variables|/Script/Engine.Character|GetMesh (Variables|Default|GetFirstPersonCharacterReference)))))
  (Variables|/Game/BG/BP/Monster/Animations/Mannequins/Animations/ABP/ABP_MTK_Player.ABP_MTK_Player_C|SetIsOnLight? _asabp_mtk_player true)
  (EventDispatchers|BindEventtoOnUseItem (Variables|Default|GetFirstPersonCharacterReference) (EventDispatchers|CreateEvent :!event Custom|OnLightProjectile)))

(event Custom|OnLightProjectile
  (CallFunction|LightServer))

(event Custom|Play%20Sound%20Multicast
  (params (Sound :type Sound%20Base%20Object%20Reference) (Location :type Vector))
  (Audio|PlaySoundatLocation Sound Location "0, 0, 0" 1.0 1.0 0.0 0 0 0 0) ; Play firing sound
)

(event Custom|LightServer
  (if (Variables|Default|GetIsLightOn?)
    (Variables|Default|SetIsLightOn? false)
    (Variables|Default|SetIsTraceOn? false)
    (else
      (Variables|Default|SetIsLightOn? true)
      (Variables|Default|SetIsTraceOn? true))))

(event EventTick
  (params (DeltaSeconds :type Float%20%28single-precision%29))
  (bind _firstpersoncharacterreference (Variables|Default|GetFirstPersonCharacterReference))
  (bind _mesh (Variables|/Script/Engine.Character|GetMesh _firstpersoncharacterreference))
  (bind _returnvalue (Math|Vector|GetForwardVector _mesh))
  (bind _returnvalue_2 (Transformation|GetWorldLocation _mesh))
  (bind _returnvalue_3 (* _returnvalue_2 _returnvalue))
  (if (Variables|Default|GetIsTraceOn?)
    (Utilities|FlowControl|Sequence
      (:then_0
        (if (< (Variables|Default|GetLightRange) 5e+02)
          (Variables|Default|SetLightRange (+ (Variables|Default|GetLightRange) 5.0))
          (Variables|Default|SetRadius (+ (Variables|Default|GetRadius) 5.0))
          (Variables|Default|SetStartLocation (+ (Variables|Default|GetStartLocation) _returnvalue_3))
          (bind _outhit (Collision|SphereTraceByChannel _returnvalue_3 (+ (Variables|Default|GetStartLocation) "0.000000,100.000000,0.000000") (Variables|Default|GetRadius) "TraceTypeQuery1" false 0 "ForDuration"))
          (if (== (Utilities|GetClass (.HitActor (Collision|BreakHitResult _outhit))) "/Game/BG/BP/AI/BP_Monster.BP_Monster_C")
            (Game|Damage|ApplyPointDamage (.HitActor (Collision|BreakHitResult _outhit)) 2e+01 (Transformation|GetActorLocation) _outhit 0 (Game|Player|GetPlayerPawn 0))
            (Development|PrintString "Hellaaaaaaaaaaaaaaaaaaaaaaaaaaaaaaaaaaa"))))
      (:then_1
        (if (not (< (Variables|Default|GetRadius) 1e+02))
          (Variables|Default|SetRadius 1.0))))))

(fn ConstructionScript)