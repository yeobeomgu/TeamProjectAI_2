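; BP_SpawnAI is a one-shot trigger actor that spawns a monster when the player enters its box.
; The overlap accepts the player character or actors tagged "player", excluding the player's LightActor.
; It spawns BP_Monster with BT_Monster at SpawnLocation, plays a spawn sound, and passes it a patrol spline and an InitialState blackboard value.
; The trigger destroys itself after a short delay.
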(event OnComponentBeginOverlap(Box)
  (params (OverlappedComponent :type Primitive%20Component%20Object%20Reference) (OtherActor :type Actor%20Object%20Reference) (OtherComp :type Primitive%20Component%20Object%20Reference) (OtherBodyIndex :type Integer) (bFromSweep :type Boolean) (SweepResult :type Hit%20Result%20Structure%20%28by%20ref%29))
  (bind _returnvalue (Game|GetPlayerCharacter 0))
  (bind _asbp_test_player (Utilities|Casting|CastToBP_TestPlayer _returnvalue))
  (if (and (!= OtherActor (Variables|/Game/BG/BP/BP_TestPlayer.BP_TestPlayer_C|GetLightActor _asbp_test_player)) (or (== OtherActor _returnvalue) (Actor|ActorHasTag OtherActor "player")))
    (Utilities|FlowControl|DoOnce (Variables|Default|GetSpawnAI?)
      (:Completed
        (bind _returnvalue_2 (AI|SpawnAIFromClass "/Game/BG/BP/AI/BP_Monster.BP_Monster_C" "/Game/BG/BP/AI/BT_Monster.BT_Monster" (Variables|Default|GetSpawnLocation) "0, 0, 0" false 0))
        (Audio|PlaySoundatLocation "/Game/BG/BP/Sound/Monster_Spawn.Monster_Spawn" (Transformation|GetActorLocation _returnvalue_2) "0, 0, 0" 1.0 1.0 0.0 0 0 0 0)
        (bind _asbp_monster (Utilities|Casting|CastToBP_Monster _returnvalue_2))
        (Variables|/Game/BG/BP/AI/BP_Monster.BP_Monster_C|SetPatrolSplinePath _asbp_monster (Variables|Default|GetPatrol%20Spline%20Path))
        (AI|Components|Blackboard|SetValueasEnum (AI|GetBlackboard _returnvalue_2) (Utilities|Name|MakeLiteralName "InitialState") (Utilities|Enum|LiteralenumMonsterInitialState "NewEnumerator1"))
        (Variables|Default|SetSpawnAI? true)
        (Utilities|FlowControl|Delay 2.0)
        (Actor|DestroyActor)))))

(event EventBeginPlay)

(event Collision|EventActorBeginOverlap
  (params (OtherActor :type Actor%20Object%20Reference)))

(event EventTick
  (params (DeltaSeconds :type Float%20%28single-precision%29)))

(fn ConstructionScript)